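; Long-shot frog enemy with flipbook animation that fires projectiles while the player is inside its box trigger.
; Tick updates the flipbook from EnemyState and attempts shots, gated by a one-second cooldown.
; Lethal damage awards score, then the flipbook update spawns a dead frog, destroys this actor and grants souls if the player has a bottle.
; BeginPlay spawns a BP_Home at its location; line-trace targeting is unconnected.
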(event `self.ReceiveTick`
  (params (DeltaSeconds :type "Float (single-precision)"))
  ;[1 1 1] Event Tick (Animation/Shooting)
  (`|ExecutionSequence`
    (:`then_0`
      (`self.Update Enemy Flipbook`))
    (:`then_1`
      (`self.Shoot`))))

(event `self.ReceiveBeginPlay`
  ;[1 1 1] Spawns Home Point for dead Frog
  (`|SpawnActorFromClass` "/Game/Blueprints/Enemies_Blueprints/BP_Home.BP_Home_C" (`KismetMathLibrary.Conv_VectorToTransform` (`SceneComponent.K2_GetComponentLocation` (`self.Capsule`))) "AdjustIfPossibleButAlwaysSpawn" "OverrideRootScale" null null))

(event `Cooldown`
  ;[1 1 1] Cool down for shooting
  (set `self.Cooldown Status` true)
  (`KismetSystemLibrary.Delay` 1.0)
  (set `self.Cooldown Status` false))

(event `/Game/Blueprints/Player_Blueprints/Interfaces/BPI_Enemy.Interact with Enemy`
  ;[1 1 1] When the player interacts with the enemy, this causes damage to the enemy
  (set `self.Health` (`KismetMathLibrary.ClampAngle` (- (`self.Health`) (`self.damage taken`)) 0.0 (`self.Default Health`)))
  (if (and (<= (`self.Health`) 0.0) (not (`self.isdead`)))
    (set `self.isdead` true)
    (bind _asbp_gamemode_base (cast `/Game/Blueprints/BP_GamemodeBase` (`GameplayStatics.GetGameMode`)))
    (`/Game/Blueprints/BP_GamemodeBase.AddTargetPoints` _asbp_gamemode_base (`self.Add Score Point`))))

(event `Shoot`
  ;[1 1 1] Can Shoot + Shoot
  (if (`self.Player in Range`)
    (if (not (`self.Cooldown Status`))
      (`self.FireProjectile`)
      (`self.Cooldown`))))

(event `EnemyDied`
  ;[1 1 1] Spawns dead version of enemy, and adds points to the player's score
  (`|SpawnActorFromClass` "/Game/Blueprints/Enemies_Blueprints/Enemies/Frog/BP_FrogDead.BP_FrogDead_C" (`SceneComponent.K2_GetComponentToWorld` (`self.Capsule`)) "Undefined" "OverrideRootScale" null null)
  (`self.K2_DestroyActor`)
  (set `self.isDead` false)
  (bind _asbp_player_s (cast `/Game/Blueprints/Player_Blueprints/BP_PlayerS` (`GameplayStatics.GetPlayerCharacter` 0)))
  (if (`/Game/Blueprints/Player_Blueprints/BP_PlayerS.Has Soul Bottle` _asbp_player_s)
    (`/Game/Blueprints/Player_Blueprints/BP_PlayerS.Add Collected Souls` _asbp_player_s)))

(event `FireProjectile`
  ;[1 1 1] Fire a projectile
  (set `self.Enemy State` "NewEnumerator4")
  (`KismetSystemLibrary.Delay` 0.3)
  (`|SpawnActorFromClass` "/Game/Blueprints/Enemies_Blueprints/Enemies/Frog/LongShotFrog/BP_FrogProjectile_2.BP_FrogProjectile_2_C" (`SceneComponent.K2_GetComponentToWorld` (`self.Capsule`)) "Undefined" "OverrideRootScale" null null)
  (`KismetSystemLibrary.Delay` 0.5)
  (set `self.Enemy State` "NewEnumerator0"))

(event `Attack Player`
  ;[1 1 1] Attacks the player when line is hit
)

(event `self.Box.OnComponentBeginOverlap`
  (params (OverlappedComponent :type "PrimitiveComponent Object Reference") (OtherActor :type "Actor Object Reference") (OtherComp :type "PrimitiveComponent Object Reference") (OtherBodyIndex :type Integer) (bFromSweep :type Boolean) (SweepResult :type "HitResult Structure (by ref)"))
  (cast `/Game/Blueprints/Player_Blueprints/BP_PlayerS` OtherActor)
  (set `self.Player in Range` true))

(event `self.Box.OnComponentEndOverlap`
  (params (OverlappedComponent :type "PrimitiveComponent Object Reference") (OtherActor :type "Actor Object Reference") (OtherComp :type "PrimitiveComponent Object Reference") (OtherBodyIndex :type Integer))
  (set `self.Player in Range` false))

(fn `Update Enemy Flipbook`
  (if (`self.isdead`)
    (`self.EnemyDied`)
    (else
      (`PaperFlipbookComponent.SetFlipbook` (`self.Sprite`) (select `/Game/Blueprints/Enemies_Blueprints/E_EnemyStates` (`self.Enemy State`) :`NewEnumerator0` (`self.Idle`) :`NewEnumerator4` (`self.Attack`) :`NewEnumerator2` (`self.Damaged`))))))

(fn `UserConstructionScript`)