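; BP_Moth is a flipbook-animated flying enemy that chases the player within range and returns to its spawned home point when the player leaves.
; Tick drives the flipbook and spawns a retreat point behind it about every two seconds, used after reaching the player or taking damage.
; Player attacks overlapping CanDamage reduce health by equipment-based amounts.
; Death awards score, spawns a falling corpse and adds souls if the player holds a bottle.
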(event `self.ReceiveBeginPlay`
  ;[1 1 1] Spawns Home Point for dead Enemy
  (bind _returnvalue (`|SpawnActorFromClass` "/Game/Blueprints/Enemies_Blueprints/BP_Home.BP_Home_C" (`KismetMathLibrary.Conv_VectorToTransform` (`SceneComponent.K2_GetComponentLocation` (`self.CapsuleComponent`))) "AdjustIfPossibleButAlwaysSpawn" "OverrideRootScale" null null))
  (set `self.Home` _returnvalue))

(event `self.canDamage.OnComponentBeginOverlap`
  (params (OverlappedComponent :type "PrimitiveComponent Object Reference") (OtherActor :type "Actor Object Reference") (OtherComp :type "PrimitiveComponent Object Reference") (OtherBodyIndex :type Integer) (bFromSweep :type Boolean) (SweepResult :type "HitResult Structure (by ref)"))
  ;[1 1 1] Damages player on collision
  (cast `/Game/Blueprints/Player_Blueprints/BP_PlayerS` OtherActor)
  (set `self.can Damage` true)
  (bind _asbp_player_s (cast `/Game/Blueprints/Player_Blueprints/BP_PlayerS` (`GameplayStatics.GetPlayerCharacter` 0)))
  ;[1 1 1] When the player interacts with the enemy, this causes damage to the enemy
  (if (`/Game/Blueprints/Player_Blueprints/BP_PlayerS.isattacking` _asbp_player_s)
    (if (`self.can Damage`)
      (if (`/Game/Blueprints/Player_Blueprints/BP_PlayerS.FireSwordStatus` _asbp_player_s)
        (set `self.Damage Taken` 35.0)
        (elif (`/Game/Blueprints/Player_Blueprints/BP_PlayerS.PurpleArmorStatus` _asbp_player_s)
          (set `self.Damage Taken` 50.0)))
      (set `self.Moth Health` (`KismetMathLibrary.ClampAngle` (- (`self.Moth Health`) (`self.damage taken`)) 0.0 (`self.Moth Default Health`)))
      (if (and (<= (`self.Moth Health`) 0.0) (not (`self.isdead`)))
        (set `self.isdead` true)
        (bind _asbp_gamemode_base (cast `/Game/Blueprints/BP_GamemodeBase` (`GameplayStatics.GetGameMode`)))
        (`/Game/Blueprints/BP_GamemodeBase.AddTargetPoints` _asbp_gamemode_base (`self.Add Score Point`))
        (else
          (set `self.gettingDamaged` true)
          (set `self.Enemy State` "NewEnumerator2")
          (`|AIMoveTo` self (0.0 0.0 0.0) (`self.NewVar_0`) 500.0
            (:`then`
              (`KismetSystemLibrary.Delay` (`PaperFlipbook.GetTotalDuration` (`self.Damaged`)))
              (set `self.gettingDamaged` false)
              (set `self.Enemy State` "NewEnumerator0"))))))))

(event `back to count`
  (bind _capsulecomponent (`self.CapsuleComponent`))
  ;[1 1 1] Spawns a point near the bat for it to return to after either taking damage or attacking the player
  (set `self.back to counter` true)
  (`KismetSystemLibrary.Delay` 2.0)
  (bind _returnvalue (`|SpawnActorFromClass` "/Game/Blueprints/Enemies_Blueprints/Enemies/Moth/DamagedSuccesfullHitLocation.DamagedSuccesfullHitLocation_C" (`KismetMathLibrary.Conv_VectorToTransform` (+ (`SceneComponent.K2_GetComponentLocation` _capsulecomponent) (* (`SceneComponent.GetForwardVector` _capsulecomponent) -200))) "Undefined" "OverrideRootScale" null null))
  (set `self.NewVar_0` _returnvalue)
  (set `self.back to counter` false))

(event `self.ReceiveTick`
  (params (DeltaSeconds :type "Float (single-precision)"))
  ;[1 1 1] Event Tick (Animation/Shooting)
  (`|ExecutionSequence`
    (:`then_0`
      (`self.Update Enemy Flipbook`))
    (:`then_1`
      (if (not (`self.back to counter`))
        (`self.back to count`)))))

(event `Chase Player`
  ;[1 1 1] Chases the player
  (`|AIMoveTo` self (0.0 0.0 0.0) (`GameplayStatics.GetPlayerCharacter` 0)
    (:`OnSuccess`
      (`KismetSystemLibrary.Delay` 0.2)
      (`|AIMoveTo` self (0.0 0.0 0.0) (`self.NewVar_0`) 0.0
        (:`OnSuccess`
          (`KismetSystemLibrary.Delay` 0.3)
          (if (`self.Player in Range`)
            (`self.Chase Player`)))))))

(event `self.inRange.OnComponentBeginOverlap`
  (params (OverlappedComponent :type "PrimitiveComponent Object Reference") (OtherActor :type "Actor Object Reference") (OtherComp :type "PrimitiveComponent Object Reference") (OtherBodyIndex :type Integer) (bFromSweep :type Boolean) (SweepResult :type "HitResult Structure (by ref)"))
  ;[1 1 1] Chasing of Player and returning to home when player escapes
  (cast `/Game/Blueprints/Player_Blueprints/BP_PlayerS` OtherActor)
  (set `self.Player in range` true)
  (`self.Chase Player`))

(event `self.inRange.OnComponentEndOverlap`
  (params (OverlappedComponent :type "PrimitiveComponent Object Reference") (OtherActor :type "Actor Object Reference") (OtherComp :type "PrimitiveComponent Object Reference") (OtherBodyIndex :type Integer))
  ;[1 1 1] Chasing of Player and returning to home when player escapes
  (cast `/Game/Blueprints/Player_Blueprints/BP_PlayerS` OtherActor)
  (set `self.Player in range` false)
  (`KismetSystemLibrary.Delay` 0.3)
  (`MovementComponent.StopMovementImmediately` (`self.CharacterMovement`))
  (`KismetSystemLibrary.Delay` 3.0)
  (`|AIMoveTo` self (0.0 0.0 0.0) (`self.Home`) 0.0))

(event `EnemyDied`
  ;[1 1 1] Spawns dead version of enemy, and adds points to the player's score
  (`|SpawnActorFromClass` "/Game/Blueprints/Enemies_Blueprints/Enemies/Moth/BP_DeadFallingMoth.BP_DeadFallingMoth_C" (`SceneComponent.K2_GetComponentToWorld` (`self.CapsuleComponent`)) "Undefined" "OverrideRootScale" null null)
  (`self.K2_DestroyActor`)
  (set `self.isDead` false)
  (bind _asbp_player_s (cast `/Game/Blueprints/Player_Blueprints/BP_PlayerS` (`GameplayStatics.GetPlayerCharacter` 0)))
  (if (`/Game/Blueprints/Player_Blueprints/BP_PlayerS.Has Soul Bottle` _asbp_player_s)
    (`/Game/Blueprints/Player_Blueprints/BP_PlayerS.Add Collected Souls` _asbp_player_s)))

(event `self.canDamage.OnComponentEndOverlap`
  (params (OverlappedComponent :type "PrimitiveComponent Object Reference") (OtherActor :type "Actor Object Reference") (OtherComp :type "PrimitiveComponent Object Reference") (OtherBodyIndex :type Integer))
  (cast `/Game/Blueprints/Player_Blueprints/BP_PlayerS` OtherActor)
  (set `self.can Damage` false))

(event `self.CapsuleComponent.OnComponentBeginOverlap`
  (params (OverlappedComponent :type "PrimitiveComponent Object Reference") (OtherActor :type "Actor Object Reference") (OtherComp :type "PrimitiveComponent Object Reference") (OtherBodyIndex :type Integer) (bFromSweep :type Boolean) (SweepResult :type "HitResult Structure (by ref)"))
  (bind _asbp_player_s (cast `/Game/Blueprints/Player_Blueprints/BP_PlayerS` OtherActor))
  (message `/Game/Blueprints/Player_Blueprints/Interfaces/BPI_Player.Interact with Player` _asbp_player_s))

(fn `Update Enemy Flipbook`
  (if (`self.isDead`)
    (`self.EnemyDied`)
    (else
      (`PaperFlipbookComponent.SetFlipbook` (`self.Sprite`) (select `/Game/Blueprints/Enemies_Blueprints/E_EnemyStates` (`self.Enemy State`) :`NewEnumerator0` (`self.Idle`) :`NewEnumerator2` (`self.Damaged`))))))

(fn `UserConstructionScript`)