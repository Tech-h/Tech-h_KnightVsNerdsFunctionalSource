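; Paper2D Shell enemy that chases and attacks the player and returns to a home point spawned at BeginPlay when they escape.
; Overlap volumes drive AIMoveTo chasing, attacks and damage taken from player swings; line-trace events exist but nothing visible triggers them.
; Tick maps EnemyState to flipbooks and polls IsDead to run death, which spawns BP_ShellDead and awards souls.
; Score is added when health runs out.
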(event `Attack Player`
  (bind _e (`self.e`))
  (bind _returnvalue (`SceneComponent.K2_GetComponentLocation` _e))
  ;[1 1 1] Attacks the player when line is hit
  (bind _outhit (`KismetSystemLibrary.LineTraceSingleForObjects` :`Start` _returnvalue :`End` (+ _returnvalue (* (`SceneComponent.GetForwardVector` _e) 300)) :`ObjectTypes` (`|MakeArray` "ObjectTypeQuery1" "ObjectTypeQuery2" "ObjectTypeQuery9" :!type "EObjectTypeQuery Enum") :`DrawDebugType` "ForDuration"))
  (bind (_bblockinghit _binitialoverlap _time _distance _location _impactpoint _normal _impactnormal _physmat _hitactor) (`GameplayStatics.BreakHitResult` _outhit))
  (if _bblockinghit
    (if (`KismetSystemLibrary.DoesImplementInterface` _hitactor "/Game/Blueprints/Player_Blueprints/Interfaces/BPI_Player.BPI_Player_C")
      (if (`self.can Damage`)
        (`self.Attack Player`)))))

(event `Front inRange`
  (bind _e (`self.e`))
  (bind _returnvalue (`SceneComponent.K2_GetComponentLocation` _e))
  (bind _outhit (`KismetSystemLibrary.LineTraceSingleForObjects` :`Start` _returnvalue :`End` (+ _returnvalue (* (`SceneComponent.GetForwardVector` _e) 800)) :`ObjectTypes` (`|MakeArray` "ObjectTypeQuery1" "ObjectTypeQuery2" "ObjectTypeQuery9" :!type "EObjectTypeQuery Enum") :`DrawDebugType` "ForDuration"))
  (bind (_bblockinghit _binitialoverlap _time _distance _location _impactpoint _normal _impactnormal _physmat _hitactor) (`GameplayStatics.BreakHitResult` _outhit))
  (if _bblockinghit
    (if (`KismetSystemLibrary.DoesImplementInterface` _hitactor "/Game/Blueprints/Player_Blueprints/Interfaces/BPI_Player.BPI_Player_C")
      (`self.Chase Player`))))

(event `self.ReceiveTick`
  (params (DeltaSeconds :type "Float (single-precision)"))
  ;[1 1 1] Event Tick (Animation/Shooting)
  (`|ExecutionSequence`
    (:`then_0`
      (`self.Update Enemy Flipbook`))))

(event `Back inRange`
  (bind _e (`self.e`))
  (bind _returnvalue (`SceneComponent.K2_GetComponentLocation` _e))
  (bind _outhit (`KismetSystemLibrary.LineTraceSingleForObjects` :`Start` _returnvalue :`End` (+ _returnvalue (* (`SceneComponent.GetForwardVector` _e) -800)) :`ObjectTypes` (`|MakeArray` "ObjectTypeQuery1" "ObjectTypeQuery2" "ObjectTypeQuery9" :!type "EObjectTypeQuery Enum") :`DrawDebugType` "ForDuration"))
  (bind (_bblockinghit _binitialoverlap _time _distance _location _impactpoint _normal _impactnormal _physmat _hitactor) (`GameplayStatics.BreakHitResult` _outhit))
  (if _bblockinghit
    (if (`KismetSystemLibrary.DoesImplementInterface` _hitactor "/Game/Blueprints/Player_Blueprints/Interfaces/BPI_Player.BPI_Player_C")
      (`self.Chase Player`))))

(event `self.ReceiveBeginPlay`
  ;[1 1 1] Spawns Home Point for dead Enemy
  (bind _returnvalue (`|SpawnActorFromClass` "/Game/Blueprints/Enemies_Blueprints/BP_Home.BP_Home_C" (`KismetMathLibrary.Conv_VectorToTransform` (`SceneComponent.K2_GetComponentLocation` (`self.CapsuleComponent`))) "AdjustIfPossibleButAlwaysSpawn" "OverrideRootScale" null null))
  (set `self.Home` _returnvalue))

(event `Cooldown`
  ;[1 1 1] Cool down countdown
  (set `self.Cooldown Status` true)
  (`KismetSystemLibrary.Delay` 1.0)
  (set `self.Cooldown Status` false))

(event `self.canDamage.OnComponentBeginOverlap`
  (params (OverlappedComponent :type "PrimitiveComponent Object Reference") (OtherActor :type "Actor Object Reference") (OtherComp :type "PrimitiveComponent Object Reference") (OtherBodyIndex :type Integer) (bFromSweep :type Boolean) (SweepResult :type "HitResult Structure (by ref)"))
  ;[1 1 1] Try's to attack player on overlap
  (cast `/Game/Blueprints/Player_Blueprints/BP_PlayerS` OtherActor)
  (set `self.can Damage` true)
  (if (`self.can Damage`)
    (`self.HitPlayer`)
    (if (`self.Cooldown Status`)
      _
      (elif (`self.can Damage`)
        (`self.HitPlayer`)))))

(event `EnemyDied`
  ;[1 1 1] Spawns dead version of enemy, and adds points to the player's score
  (`PrimitiveComponent.SetCollisionEnabled` (`self.CapsuleComponent`) "NoCollision")
  (`KismetSystemLibrary.Delay` (`PaperFlipbook.GetTotalDuration` (`self.Death`)))
  (`|SpawnActorFromClass` "/Game/Blueprints/Enemies_Blueprints/Enemies/Shell/BP_ShellDead.BP_ShellDead_C" (`SceneComponent.K2_GetComponentToWorld` (`self.CapsuleComponent`)) "Undefined" "OverrideRootScale" null null)
  (`self.K2_DestroyActor`)
  (set `self.isDead` false)
  (bind _asbp_player_s (cast `/Game/Blueprints/Player_Blueprints/BP_PlayerS` (`GameplayStatics.GetPlayerCharacter` 0)))
  (if (`/Game/Blueprints/Player_Blueprints/BP_PlayerS.Has Soul Bottle` _asbp_player_s)
    (`/Game/Blueprints/Player_Blueprints/BP_PlayerS.Add Collected Souls` _asbp_player_s)))

(event `self.canDamage.OnComponentEndOverlap`
  (params (OverlappedComponent :type "PrimitiveComponent Object Reference") (OtherActor :type "Actor Object Reference") (OtherComp :type "PrimitiveComponent Object Reference") (OtherBodyIndex :type Integer))
  ;[1 1 1] Try's to attack player on overlap
  (set `self.can Damage` false))

(event `HitPlayer`
  ;[1 1 1] Attacking Player
  (set `self.Enemy State` "NewEnumerator4")
  (`KismetSystemLibrary.Delay` (`PaperFlipbook.GetTotalDuration` (`self.Attack`)))
  (bind _asbp_player_s (cast `/Game/Blueprints/Player_Blueprints/BP_PlayerS` (`GameplayStatics.GetPlayerCharacter` 0)))
  (set `/Game/Blueprints/Player_Blueprints/BP_PlayerS.KnightorFrog?` true _asbp_player_s)
  (if (`self.can Damage`)
    (message `/Game/Blueprints/Player_Blueprints/Interfaces/BPI_Player.Interact with Player` _asbp_player_s)
    (set `self.Enemy State` "NewEnumerator0")))

(event `Chase Player`
  ;[1 1 1] Chases the player
  (set `self.Enemy State` "NewEnumerator1")
  (`|AIMoveTo` self (0.0 0.0 0.0) (`GameplayStatics.GetPlayerCharacter` 0) 150.0
    (:`OnSuccess`
      (if (not (`self.can Damage`))
        (`self.Chase Player`)))))

(event `self.Box.OnComponentBeginOverlap`
  (params (OverlappedComponent :type "PrimitiveComponent Object Reference") (OtherActor :type "Actor Object Reference") (OtherComp :type "PrimitiveComponent Object Reference") (OtherBodyIndex :type Integer) (bFromSweep :type Boolean) (SweepResult :type "HitResult Structure (by ref)"))
  ;[1 1 1] When the player interacts with the enemy, this causes damage to the enemy
  (cast `/Game/Blueprints/Player_Blueprints/BP_PlayerS` OtherActor)
  (set `self.NewVar_0` true)
  (bind _asbp_player_s (cast `/Game/Blueprints/Player_Blueprints/BP_PlayerS` (`GameplayStatics.GetPlayerCharacter` 0)))
  (if (`/Game/Blueprints/Player_Blueprints/BP_PlayerS.isattacking` _asbp_player_s)
    (if (`self.NewVar_0`)
      (if (`/Game/Blueprints/Player_Blueprints/BP_PlayerS.FireSwordStatus` _asbp_player_s)
        (set `self.Damage Taken` 50.0)
        (elif (`/Game/Blueprints/Player_Blueprints/BP_PlayerS.PurpleArmorStatus` _asbp_player_s)
          (set `self.Damage Taken` 50.0)
          (else
            (set `self.Damage Taken` 40.0))))
      (set `self.Health` (`KismetMathLibrary.ClampAngle` (- (`self.Health`) (`self.damage taken`)) 0.0 (`self.Default Health`)))
      (if (and (<= (`self.Health`) 0.0) (not (`self.isdead`)))
        (set `self.isdead` true)
        (bind _asbp_gamemode_base (cast `/Game/Blueprints/BP_GamemodeBase` (`GameplayStatics.GetGameMode`)))
        (`/Game/Blueprints/BP_GamemodeBase.AddTargetPoints` _asbp_gamemode_base (`self.Add Score Point`))
        (else
          (set `self.gettingDamaged` true)
          (set `self.Enemy State` "NewEnumerator2")
          (`KismetSystemLibrary.Delay` (`PaperFlipbook.GetTotalDuration` (`self.Damaged`)))
          (set `self.gettingDamaged` false)
          (set `self.Enemy State` "NewEnumerator0"))))))

(event `self.inRange.OnComponentBeginOverlap`
  (params (OverlappedComponent :type "PrimitiveComponent Object Reference") (OtherActor :type "Actor Object Reference") (OtherComp :type "PrimitiveComponent Object Reference") (OtherBodyIndex :type Integer) (bFromSweep :type Boolean) (SweepResult :type "HitResult Structure (by ref)"))
  ;[1 1 1] Chasing of Player and returning to home when player escapes
  (cast `/Game/Blueprints/Player_Blueprints/BP_PlayerS` OtherActor)
  (set `self.Player in range` true)
  (`self.Chase Player`))

(event `self.Box.OnComponentEndOverlap`
  (params (OverlappedComponent :type "PrimitiveComponent Object Reference") (OtherActor :type "Actor Object Reference") (OtherComp :type "PrimitiveComponent Object Reference") (OtherBodyIndex :type Integer))
  (cast `/Game/Blueprints/Player_Blueprints/BP_PlayerS` OtherActor)
  (set `self.NewVar_0` false))

(event `self.inRange.OnComponentEndOverlap`
  (params (OverlappedComponent :type "PrimitiveComponent Object Reference") (OtherActor :type "Actor Object Reference") (OtherComp :type "PrimitiveComponent Object Reference") (OtherBodyIndex :type Integer))
  ;[1 1 1] Chasing of Player and returning to home when player escapes
  (cast `/Game/Blueprints/Player_Blueprints/BP_PlayerS` OtherActor)
  (set `self.Player in range` false)
  (`MovementComponent.StopMovementImmediately` (`self.CharacterMovement`))
  (set `self.Enemy State` "NewEnumerator0")
  (`KismetSystemLibrary.Delay` 4.0)
  (set `self.Enemy State` "NewEnumerator1")
  (`|AIMoveTo` self (0.0 0.0 0.0) (`self.Home`) 0.0
    (:`then`
      (set `self.Enemy State` "NewEnumerator0"))))

(fn `Update Enemy Flipbook`
  (if (`self.isDead`)
    (`PaperFlipbookComponent.SetFlipbook` (`self.Sprite`) (`self.Death`))
    (`self.EnemyDied`)
    (else
      (`PaperFlipbookComponent.SetFlipbook` (`self.Sprite`) (select `/Game/Blueprints/Enemies_Blueprints/E_EnemyStates` (`self.Enemy State`) :`NewEnumerator0` (`self.Idle`) :`NewEnumerator1` (`self.Walk`) :`NewEnumerator4` (`self.Attack`) :`NewEnumerator2` (`self.Damaged`))))))

(fn `UserConstructionScript`)