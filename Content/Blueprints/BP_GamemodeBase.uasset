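; Base game mode Blueprint that tracks score and kills and runs a five-second timer for a minilevel.
; On BeginPlay it sets the fullscreen mode to windowed, without applying the settings.
; An event adds points to the target score and increments the kill count.
; The timer loops on short delays until five seconds accumulate, then opens LevelThree and sets the OrcKey flag on the varsInstance game instance.
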(event `self.ReceiveBeginPlay`
  (bind _returnvalue (`GameUserSettings.GetGameUserSettings`))
  (`GameUserSettings.SetFullscreenMode` _returnvalue "Windowed")
  (`KismetSystemLibrary.Delay` 1.0))

(event `AddTargetPoints`
  (params (`Add score point` :type "Float (double-precision)"))
  (set `self.TargetScore` (+ `Add score point` (`self.TargetScore`)))
  (set `self.GamemodeKills` (+ (`self.GamemodeKills`) 1.0)))

(event `5 Second Timer (for minilevel)`
  (bind _time__5sec_ (`self.Time (5sec)`))
  (`KismetSystemLibrary.Delay` 0.1)
  (set `self.Time (5sec)` (+ _time__5sec_ 0.1))
  (if (>= _time__5sec_ 5.0)
    (`GameplayStatics.OpenLevel` "LevelThree")
    (bind _asvars_instance (cast `/Game/Blueprints/varsInstance` (`GameplayStatics.GetGameInstance`)))
    (set `/Game/Blueprints/varsInstance.OrcKey` true _asvars_instance)
    (else
      (`self.5 Second Timer (for minilevel)`))))

(fn `UserConstructionScript`)