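; BP_Collection is a soul well interactable that opens a gate once the player brings enough souls.
; Player overlap either grants the soul bottle or, if already held, compares its soul count to the requirement read from the varsInstance game instance.
; Success fires once: it plays sounds, swaps activation flipbooks, removes the bottle widget, sets GotSouls, and disables Box1 collision after a delay.
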(event `self.ReceiveBeginPlay`
  ;[1 1 1] Sets the number of souls required to active the soul well
  (bind _asvars_instance (cast `/Game/Blueprints/varsInstance` (`GameplayStatics.GetGameInstance`)))
  (set `self.Souls Required` (`/Game/Blueprints/varsInstance.SoulsRequired` _asvars_instance)))

(event `self.Interactive Collider.OnComponentBeginOverlap`
  (params (OverlappedComponent :type "PrimitiveComponent Object Reference") (OtherActor :type "Actor Object Reference") (OtherComp :type "PrimitiveComponent Object Reference") (OtherBodyIndex :type Integer) (bFromSweep :type Boolean) (SweepResult :type "HitResult Structure (by ref)"))
  ;[1 1 1] Soul number calculation
  (bind _asbp_player_s (cast `/Game/Blueprints/Player_Blueprints/BP_PlayerS` OtherActor))
  (if (`/Game/Blueprints/Player_Blueprints/BP_PlayerS.Has Soul Bottle` _asbp_player_s)
    (set `self.NumberOfSoulsRN` (`/Game/Blueprints/Player_Blueprints/BP_PlayerS.Number of Souls` _asbp_player_s))
    (`self.Check SoulCont`)
    (else
      (set `/Game/Blueprints/Player_Blueprints/BP_PlayerS.Has Soul Bottle` true _asbp_player_s))))

(event `Flipbook change`
  ;[1 1 1] Sets activation flipbooks (offests to compensate for flipbook size)
  (if (not (`self.Played`))
    (`PaperFlipbookComponent.SetFlipbook` (`self.PaperFlipbook`) "/Game/Assets/Art/Flipbooks/Dungeon_Flipbooks/SoulJacuzzi_Flipbooks/FB_Activating_SoulJacuzzi.FB_Activating_SoulJacuzzi")
    (`KismetSystemLibrary.Delay` (`PaperFlipbookComponent.GetFlipbookLength` (`self.PaperFlipbook`)))
    (`PaperFlipbookComponent.SetFlipbook` (`self.PaperFlipbook`) "/Game/Assets/Art/Flipbooks/Dungeon_Flipbooks/SoulJacuzzi_Flipbooks/FB_Activated_SoulJucuzzi.FB_Activated_SoulJucuzzi")
    (set `self.Played` true)
    (bind _asvars_instance (cast `/Game/Blueprints/varsInstance` (`GameplayStatics.GetGameInstance`)))
    (`Widget.RemoveFromParent` (`/Game/Blueprints/varsInstance.WBP_SoulBottle` _asvars_instance))))

(event `Check SoulCont`
  ;[1 1 1] Checks soul count + opens doors
  (if (>= (`self.NumberOfSoulsRN`) (`self.Souls Required`))
    (`/Engine/EditorBlueprintResources/StandardMacros.DoOnce` false
      (:`Completed`
        (`GameplayStatics.PlaySoundAtLocation` "/Game/Assets/Music/Soul_JacuzziCue.Soul_JacuzziCue" (0.0 0.0 0.0) (struct) 1.0 1.0 0.0 null null null)
        (`self.Flipbook change`)
        (bind _asvars_instance (cast `/Game/Blueprints/varsInstance` (`GameplayStatics.GetGameInstance`)))
        (set `/Game/Blueprints/varsInstance.GotSouls` true _asvars_instance)
        (`KismetSystemLibrary.Delay` 4.0)
        (`GameplayStatics.PlaySoundAtLocation` "/Game/Assets/Music/GateOpening_Cue.GateOpening_Cue" (0.0 0.0 0.0) (struct) 1.0 1.0 0.0 null null null)
        (`PrimitiveComponent.SetCollisionEnabled` (`self.Box1`) "NoCollision")))))

(fn `UserConstructionScript`
  (`PaperFlipbookComponent.SetLooping` (`self.PaperFlipbook`) (`self.AutoPlay`)))