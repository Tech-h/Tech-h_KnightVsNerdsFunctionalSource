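; BP_DyingComrade is a one-time trigger interactable that gives the player the soul bottle.
; When BP_PlayerS overlaps its Box, it halts the player's current movement and calls SetFBs.
; SetFBs sets the player's HasSoulBottle flag and shows the WBP_GetSoulsForWell_Prt_1 widget on the player screen.
; The Box then disables its collision so the event cannot repeat.
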(event `self.Box.OnComponentBeginOverlap`
  (params (OverlappedComponent :type "PrimitiveComponent Object Reference") (OtherActor :type "Actor Object Reference") (OtherComp :type "PrimitiveComponent Object Reference") (OtherBodyIndex :type Integer) (bFromSweep :type Boolean) (SweepResult :type "HitResult Structure (by ref)"))
  (bind _asbp_player_s (cast `/Game/Blueprints/Player_Blueprints/BP_PlayerS` OtherActor))
  (bind _output_get (set `self.As BP Player S` _asbp_player_s))
  (`MovementComponent.StopMovementImmediately` (`Character.CharacterMovement` _output_get))
  (`self.SetFBs`)
  (`PrimitiveComponent.SetCollisionEnabled` (`self.Box`) "NoCollision"))

(event `SetFBs`
  (set `/Game/Blueprints/Player_Blueprints/BP_PlayerS.Has Soul Bottle` true (`self.As BP Player S`))
  (bind _returnvalue (`|CreateWidget` "/Game/Blueprints/UI_Blueprints/Instructions/WBP_GetSoulsForWell_Prt_1.WBP_GetSoulsForWell_Prt_1_C"))
  (`UserWidget.AddToPlayerScreen` _returnvalue 0))

(fn `UserConstructionScript`)