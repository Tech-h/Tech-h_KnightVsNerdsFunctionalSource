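; Interactable ladder that teleports the player between its top and bottom instead of climbing.
; Overlaps on the two base collisions set ladder flags and toggle FBE1 or FBE2 visibility.
; On interact, OnBottomLadder picks the destination collision's transform; if the stored overlap actor is the player, control rotation follows the character and velocity zeroes.
; The construction script positions teleport point components from location variables, though interaction does not use them.
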(event `/Game/Blueprints/Player_Blueprints/Interfaces/BPI_Interact.Interact with Object`
  (bind _returnvalue (`GameplayStatics.GetPlayerCharacter` 0))
  (bind _returnvalue_2 (`GameplayStatics.GetPlayerCharacter` 0))
  (bind (_returnvalue_location _returnvalue_rotation) (`KismetMathLibrary.BreakTransform` (`SceneComponent.K2_GetComponentToWorld` (`self.Bottom Base Collision`))))
  (bind (_returnvalue_location_2 _returnvalue_rotation_2) (`KismetMathLibrary.BreakTransform` (`SceneComponent.K2_GetComponentToWorld` (`self.Top Base Collision`))))
  ;[1 1 1] Teleports the player up
  (if (`self.On Bottom Ladder`)
    (bind _asbp_player_s (cast `/Game/Blueprints/Player_Blueprints/BP_PlayerS` (`GameplayStatics.GetPlayerCharacter` 0)))
    (`SceneComponent.K2_SetWorldTransform` (`Actor.RootComponent` _asbp_player_s) (`KismetMathLibrary.MakeTransform` _returnvalue_location_2 _returnvalue_rotation_2) false false)
    (if (== (`self.Other Actor (Bottom)`) _returnvalue_2)
      (`Controller.SetControlRotation` (`GameplayStatics.GetPlayerController` 0) (`self.K2_GetActorRotation` _returnvalue_2))
      (set `MovementComponent.Velocity` (0.0 0.0 0.0) (`Character.CharacterMovement` _returnvalue_2)))
    (else
      (bind _asbp_player_s_2 (cast `/Game/Blueprints/Player_Blueprints/BP_PlayerS` (`GameplayStatics.GetPlayerCharacter` 0)))
      (`SceneComponent.K2_SetWorldTransform` (`Actor.RootComponent` _asbp_player_s_2) (`KismetMathLibrary.MakeTransform` _returnvalue_location _returnvalue_rotation) false false)
      (if (== (`self.Other Actor (Top)`) _returnvalue)
        (`Controller.SetControlRotation` (`GameplayStatics.GetPlayerController` 0) (`self.K2_GetActorRotation` _returnvalue))
        (set `MovementComponent.Velocity` (0.0 0.0 0.0) (`Character.CharacterMovement` _returnvalue))))))

(event `self.Bottom Base Collision.OnComponentBeginOverlap`
  (params (OverlappedComponent :type "PrimitiveComponent Object Reference") (OtherActor :type "Actor Object Reference") (OtherComp :type "PrimitiveComponent Object Reference") (OtherBodyIndex :type Integer) (bFromSweep :type Boolean) (SweepResult :type "HitResult Structure (by ref)"))
  ;[1 1 1] Sets if Colliding with ladder hitbox
  (set `self.Other Actor (Bottom)` OtherActor)
  (set `self.onLadder` true)
  (set `self.On Bottom Ladder` true)
  (`SceneComponent.SetHiddenInGame` (`self.FB_e_1`) false false))

(event `self.Bottom Base Collision.OnComponentEndOverlap`
  (params (OverlappedComponent :type "PrimitiveComponent Object Reference") (OtherActor :type "Actor Object Reference") (OtherComp :type "PrimitiveComponent Object Reference") (OtherBodyIndex :type Integer))
  ;[1 1 1] Sets if not colliding with ladder hitbox
  (set `self.onLadder` false)
  (set `self.On Bottom Ladder` false)
  (`SceneComponent.SetHiddenInGame` (`self.FB_e_1`) true false))

(event `self.Top Base Collision.OnComponentBeginOverlap`
  (params (OverlappedComponent :type "PrimitiveComponent Object Reference") (OtherActor :type "Actor Object Reference") (OtherComp :type "PrimitiveComponent Object Reference") (OtherBodyIndex :type Integer) (bFromSweep :type Boolean) (SweepResult :type "HitResult Structure (by ref)"))
  ;[1 1 1] Sets if collising with top base ladder hitbox
  (set `self.Other Actor (Top)` OtherActor)
  (set `self.onLadder` true)
  (`SceneComponent.SetHiddenInGame` (`self.FB_e_2`) false false))

(event `self.Top Base Collision.OnComponentEndOverlap`
  (params (OverlappedComponent :type "PrimitiveComponent Object Reference") (OtherActor :type "Actor Object Reference") (OtherComp :type "PrimitiveComponent Object Reference") (OtherBodyIndex :type Integer))
  ;[1 1 1] Sets if colliding with top base ladder hitbox
  (set `self.onLadder` false)
  (`SceneComponent.SetHiddenInGame` (`self.FB_e_2`) true false))

(fn `UserConstructionScript`
  (`SceneComponent.K2_SetRelativeTransform` (`self.Top Teleport point`) (`self.Top Teleport Location`) false false)
  (`SceneComponent.K2_SetRelativeTransform` (`self.Bottom Teleport point`) (`self.Bottom Teleport Location`) false false))