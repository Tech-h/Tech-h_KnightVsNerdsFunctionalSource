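; BP_OrcDoor is an interactable door that tracks whether a player holding the orc key is standing at it.
; Overlapping its Box reveals the E component, then reads OrcKey from the varsInstance game instance and sets OnOrcDoor if true.
; Ending the overlap hides E and clears the flag.
; The overlapping actor is not filtered, and the door's opening is not handled in this Blueprint.
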(event `self.Box.OnComponentBeginOverlap`
  (params (OverlappedComponent :type "PrimitiveComponent Object Reference") (OtherActor :type "Actor Object Reference") (OtherComp :type "PrimitiveComponent Object Reference") (OtherBodyIndex :type Integer) (bFromSweep :type Boolean) (SweepResult :type "HitResult Structure (by ref)"))
  (`SceneComponent.SetHiddenInGame` (`self.e`) false false)
  ;[1 1 1] Checks if orc key is present
  (bind _asvars_instance (cast `/Game/Blueprints/varsInstance` (`GameplayStatics.GetGameInstance`)))
  (if (`/Game/Blueprints/varsInstance.OrcKey` _asvars_instance)
    (set `self.OnOrcDoor` true)))

(event `self.Box.OnComponentEndOverlap`
  (params (OverlappedComponent :type "PrimitiveComponent Object Reference") (OtherActor :type "Actor Object Reference") (OtherComp :type "PrimitiveComponent Object Reference") (OtherBodyIndex :type Integer))
  (`SceneComponent.SetHiddenInGame` (`self.e`) true false)
  (set `self.OnOrcDoor` false))

(fn `UserConstructionScript`)