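; BP_PrisonNPC is an interactable prison NPC that serves as an entry point to a mini level, judging by the widget it opens.
; A Box overlap with BP_PlayerS shows PaperFlipbook1, apparently an interaction prompt, and leaving hides it again; the construction script starts it hidden.
; InteractwithObject waits briefly, then creates WBP_TravelingToMiniLevel and adds it to the viewport.
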(event `self.Box.OnComponentBeginOverlap`
  (params (OverlappedComponent :type "PrimitiveComponent Object Reference") (OtherActor :type "Actor Object Reference") (OtherComp :type "PrimitiveComponent Object Reference") (OtherBodyIndex :type Integer) (bFromSweep :type Boolean) (SweepResult :type "HitResult Structure (by ref)"))
  (cast `/Game/Blueprints/Player_Blueprints/BP_PlayerS` OtherActor)
  (`SceneComponent.SetHiddenInGame` (`self.PaperFlipbook1`) false false))

(event `self.Box.OnComponentEndOverlap`
  (params (OverlappedComponent :type "PrimitiveComponent Object Reference") (OtherActor :type "Actor Object Reference") (OtherComp :type "PrimitiveComponent Object Reference") (OtherBodyIndex :type Integer))
  (cast `/Game/Blueprints/Player_Blueprints/BP_PlayerS` OtherActor)
  (`SceneComponent.SetHiddenInGame` (`self.PaperFlipbook1`) true false))

(event `/Game/Blueprints/Player_Blueprints/Interfaces/BPI_Interact.Interact with Object`
  (`KismetSystemLibrary.Delay` 0.2)
  (bind _returnvalue (`|CreateWidget` "/Game/Blueprints/UI_Blueprints/Instructions/WBP_TravelingToMiniLevel.WBP_TravelingToMiniLevel_C"))
  (`UserWidget.AddToViewport` _returnvalue 0))

(fn `UserConstructionScript`
  (`SceneComponent.SetHiddenInGame` (`self.PaperFlipbook1`) true false))